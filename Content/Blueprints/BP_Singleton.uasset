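; BP_Singleton is a save manager that persists collected objects, such as coins, per level.
; Save writes AlreadyCollectedObjects into an SG_Object save in a slot named after the current level, reusing any existing save.
; Load waits briefly, clears that array and destroys each actor referenced in the saved Coins, without refilling the array.
; DeleteSave removes the current level's slot, and debug prints trace the operations.
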(event Custom|Load
  (Utilities|FlowControl|Delay 0.2)
  (Development|PrintString (Utilities|String|Append "Starting load level" (stale _returnvalue) "Wish me luck"))
  ;[0 0.4171 1] LoadGame
  (Utilities|Array|Clear (Variables|Default|GetAlready%20Collected%20Objects))
  (bind _returnvalue (Game|GetCurrentLevelName true))
  (bind _returnvalue_2 (SaveGame|DoesSaveGameExist _returnvalue))
  (if _returnvalue_2
    (bind _returnvalue_3 (SaveGame|LoadGamefromSlot _returnvalue))
    (bind _assg_object (Utilities|Casting|CastToSG_Object _returnvalue_3))
    (Variables|Default|SetAs%20SG%20Object _assg_object)
    (for _array_element (Variables|/Game/Blueprints/SG_Object.SG_Object_C|GetCoins _assg_object)
      (Actor|DestroyActor _array_element))))

(event Custom|Delete%20Save
  (bind _returnvalue (Game|GetCurrentLevelName true))
  (bind _returnvalue_2 (SaveGame|DoesSaveGameExist _returnvalue))
  (if _returnvalue_2
    (SaveGame|DeleteGameinSlot _returnvalue)
    (Development|PrintString "save deleted")
    (else
      (Development|PrintString "no game save "))))

(event Custom|Save
  (Development|PrintString "Hello")
  (bind _returnvalue (Game|GetCurrentLevelName true))
  (bind _returnvalue_2 (SaveGame|DoesSaveGameExist _returnvalue))
  (if _returnvalue_2
    (bind _returnvalue_3 (SaveGame|LoadGamefromSlot _returnvalue))
    (Variables|Default|SetSaver%20Subclass _returnvalue_3)
    (else
      (bind _returnvalue_4 (SaveGame|CreateSaveGameObject "/Game/Blueprints/SG_Object.SG_Object_C"))
      (Variables|Default|SetSaver%20Subclass _returnvalue_4)))
  (bind _assg_object (Utilities|Casting|CastToSG_Object (Variables|Default|GetSaver%20Subclass))
    (:then
      (Variables|/Game/Blueprints/SG_Object.SG_Object_C|SetCoins _assg_object (Variables|Default|GetAlready%20Collected%20Objects))
      (bind _returnvalue_5 (Game|GetCurrentLevelName true))
      (SaveGame|SaveGametoSlot _assg_object _returnvalue_5)
      (Development|PrintString "save successful"))
    (:CastFailed
      (Development|PrintString "boink"))))